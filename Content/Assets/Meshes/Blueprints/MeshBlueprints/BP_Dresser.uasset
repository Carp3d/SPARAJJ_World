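; BP_Dresser is a dresser actor that populates itself with six separate BP_Drawer actors when play begins.
; On BeginPlay, a sequence spawns each drawer at the dresser's transform and attaches it to one of six slot components in a top and bottom, left, middle and right grid.
; Attachment snaps location and rotation to the slot while keeping world scale, and the construction script is empty.
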(event EventBeginPlay
  (Utilities|FlowControl|Sequence
    (:then_0
      (bind _returnvalue (Game|SpawnActorfromClass "/Game/Assets/Meshes/Blueprints/MeshBlueprints/BP_Drawer.BP_Drawer_C" (Transformation|GetActorTransform) "Undefined" 0 0))
      (Transformation|AttachComponentToComponent _returnvalue (Variables|Default|GetTopLeft) "None" "SnapToTarget" "SnapToTarget" "KeepWorld" true))
    (:then_1
      (bind _returnvalue_2 (Game|SpawnActorfromClass "/Game/Assets/Meshes/Blueprints/MeshBlueprints/BP_Drawer.BP_Drawer_C" (Transformation|GetActorTransform) "Undefined" 0 0))
      (Transformation|AttachComponentToComponent _returnvalue_2 (Variables|Default|GetBottomLeft) "None" "SnapToTarget" "SnapToTarget" "KeepWorld" true))
    (:then_2
      (bind _returnvalue_3 (Game|SpawnActorfromClass "/Game/Assets/Meshes/Blueprints/MeshBlueprints/BP_Drawer.BP_Drawer_C" (Transformation|GetActorTransform) "Undefined" 0 0))
      (Transformation|AttachComponentToComponent _returnvalue_3 (Variables|Default|GetTopMiddle) "None" "SnapToTarget" "SnapToTarget" "KeepWorld" true))
    (:then_3
      (bind _returnvalue_4 (Game|SpawnActorfromClass "/Game/Assets/Meshes/Blueprints/MeshBlueprints/BP_Drawer.BP_Drawer_C" (Transformation|GetActorTransform) "Undefined" 0 0))
      (Transformation|AttachComponentToComponent _returnvalue_4 (Variables|Default|GetBottomMiddle) "None" "SnapToTarget" "SnapToTarget" "KeepWorld" true))
    (:then_4
      (bind _returnvalue_5 (Game|SpawnActorfromClass "/Game/Assets/Meshes/Blueprints/MeshBlueprints/BP_Drawer.BP_Drawer_C" (Transformation|GetActorTransform) "Undefined" 0 0))
      (Transformation|AttachComponentToComponent _returnvalue_5 (Variables|Default|GetTopRight) "None" "SnapToTarget" "SnapToTarget" "KeepWorld" true))
    (:then_5
      (bind _returnvalue_6 (Game|SpawnActorfromClass "/Game/Assets/Meshes/Blueprints/MeshBlueprints/BP_Drawer.BP_Drawer_C" (Transformation|GetActorTransform) "Undefined" 0 0))
      (Transformation|AttachComponentToComponent _returnvalue_6 (Variables|Default|GetBottomRight) "None" "SnapToTarget" "SnapToTarget" "KeepWorld" true))))

(fn ConstructionScript)