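; BP_Pedestal is an interactable pedestal that takes a required number of idols from the player and spawns an idol on itself.
; Its Interact event checks the ThirdPersonCharacter's Idol count against NumberofIdolsNeeded.
; Once the count suffices, a DoOnce spawns BP_Idol at an offset from the mesh, clears that actor's Idol variable, deducts the cost and prints a debug string.
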(event EventInteract
  (bind _numberofidolsneeded (Variables|Default|GetNumberofIdolsNeeded))
  ;[1 1 1] Event Interact
  (bind _asthird_person_character (Utilities|Casting|CastToThirdPersonCharacter (Game|GetPlayerCharacter 0)))
  (if (>= (Variables|/Game/ThirdPersonBP/Blueprints/ThirdPersonCharacter.ThirdPersonCharacter_C|GetIdol _asthird_person_character) _numberofidolsneeded)
    (Utilities|FlowControl|DoOnce false
      (:Completed
        (bind _returnvalue (Game|SpawnActorfromClass "/Game/Assets/Meshes/Blueprints/MeshBlueprints/BP_Idol.BP_Idol_C" (Math|Transform|MakeTransform (+ (Variables|Default|GetPickupOffset) (Transformation|GetWorldLocation (Variables|Default|GetStaticMesh)))) "Undefined" 0 0))
        (Variables|/Game/Assets/Meshes/Blueprints/MeshBlueprints/BP_Idol.BP_Idol_C|SetIdol _returnvalue 0)
        (Variables|/Game/ThirdPersonBP/Blueprints/ThirdPersonCharacter.ThirdPersonCharacter_C|SetIdol _asthird_person_character (- (Variables|/Game/ThirdPersonBP/Blueprints/ThirdPersonCharacter.ThirdPersonCharacter_C|GetIdol _asthird_person_character) _numberofidolsneeded))
        (Development|PrintString "Hello")))))

(fn ConstructionScript)