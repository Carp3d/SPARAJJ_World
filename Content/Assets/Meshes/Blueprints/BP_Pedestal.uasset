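; BP_Pedestal is an interactable pedestal that spawns an idol the first time it receives the Interact event.
; Interact checks that the player is a ThirdPersonCharacter, then passes through a DoOnce that is never reset.
; It spawns a BP_Idol at the static mesh's world location plus PickupOffset, sets that idol's Idol variable to None and prints a debug string.
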(event EventInteract
  ;[1 1 1] Event Interact
  (Utilities|Casting|CastToThirdPersonCharacter (Game|GetPlayerCharacter 0))
  (Utilities|FlowControl|DoOnce false
    (:Completed
      (bind _returnvalue (Game|SpawnActorfromClass "/Game/Assets/Meshes/Blueprints/BP_Idol.BP_Idol_C" (Math|Transform|MakeTransform (+ (Variables|Default|GetPickupOffset) (Transformation|GetWorldLocation (Variables|Default|GetStaticMesh)))) "Undefined" 0 0))
      (Variables|/Game/Assets/Meshes/Blueprints/BP_Idol.BP_Idol_C|SetIdol _returnvalue 0)
      (Development|PrintString "Hello"))))

(fn ConstructionScript)